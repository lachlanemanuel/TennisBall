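; Backup of older tennis game logic that moves a ball between two players via their aim targets.
; Each player's hit event chains two timelines, lerping the non-simulated ball from hitter to aim target, then to the opponent's position target, though both play rates are set to zero.
; Launch functions compute arc velocities from gravity and max height but are never called here; AddForce attempts and stray math nodes are left disconnected.
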(event Custom|Player_02_Hit
  (bind _tennisball (Variables|Default|GetTennisBall))
  (bind _player_02_aimtarget (Variables|Default|GetPlayer_02_AimTarget))
  (bind _returnvalue (Transformation|GetWorldLocation _player_02_aimtarget))
  ;[1 1 1] Less Terrible
  (Components|Timeline|SetPlayRate (Variables|Default|GetPlayer02%20Hit) 0.0)
  (Components|Timeline|SetPlayRate (Variables|Default|GetPlayer02%20Bounce) 0.0)
  (bind _before_bounce (Timeline|Player02%20Hit Play)
    (:Update
      (Transformation|SetWorldLocation _tennisball (Math|Vector|Lerp(Vector) (Transformation|GetWorldLocation (Variables|Default|GetPlayer_02)) _returnvalue _before_bounce) false false))
    (:Finished
      (bind _after_bounce (Timeline|Player02%20Bounce Play)
        (:Update
          (Transformation|SetWorldLocation _tennisball (Math|Vector|Lerp(Vector) _returnvalue (Transformation|GetWorldLocation (Variables|Default|GetPlayer_01_PositionTarget)) _after_bounce) false false))))))

(event Custom|Player_01%20Hit
  (bind _tennisball (Variables|Default|GetTennisBall))
  (bind _player_01_aimtarget (Variables|Default|GetPlayer_01_AimTarget))
  (bind _returnvalue (Transformation|GetWorldLocation _player_01_aimtarget))
  ;[1 1 1] Less Terrible
  (Components|Timeline|SetPlayRate (Variables|Default|GetPlayer01%20Hit) 0.0)
  (Components|Timeline|SetPlayRate (Variables|Default|GetPlayer01%20Bounce) 0.0)
  (bind _before_bounce (Timeline|Player01%20Hit Play)
    (:Update
      (Transformation|SetWorldLocation _tennisball (Math|Vector|Lerp(Vector) (Transformation|GetWorldLocation (Variables|Default|GetPlayer_01)) _returnvalue _before_bounce) false false))
    (:Finished
      (bind _after_bounce (Timeline|Player01%20Bounce Play)
        (:Update
          (Transformation|SetWorldLocation _tennisball (Math|Vector|Lerp(Vector) _returnvalue (Transformation|GetWorldLocation (Variables|Default|GetPlayer_02_PositionTarget)) _after_bounce) false false))))))

(event EventBeginPlay
  (Physics|SetSimulatePhysics (Variables|Default|GetTennisBall) false))

(fn ConstructionScript)

(fn Player01Launch
  (bind _tennisball (Variables|Default|GetTennisBall))
  (bind _ball_max_height (Variables|Exposed|GetBall%20Max%20Height))
  (bind _player_01_aimtarget (Variables|Default|GetPlayer_01_AimTarget))
  (bind _gravity (Variables|Math|GetGravity))
  (bind _returnvalue (Transformation|GetWorldLocation _player_01_aimtarget))
  (bind _returnvalue_2 (Transformation|GetWorldLocation _tennisball))
  (LocalVariables|SetZdisplacement (- (.z _returnvalue) (.z _returnvalue_2)))
  (LocalVariables|SetXYdisplacement (Math|Vector|MakeVector (- (.x _returnvalue) (.x _returnvalue_2)) (- (.y _returnvalue) (.y _returnvalue_2)) 0.0))
  (bind _output_get (LocalVariables|SetZVelocity (* (Math|Vector|VectorUp) (Math|Float|Sqrt (|(((0-2)*g)*h) _gravity _ball_max_height)))))
  (bind _output_get_2 (LocalVariables|SetXYVelocity (/ (LocalVariables|GetXYdisplacement) (+ (Math|Float|Sqrt (|(((0-2)*h)/g) _gravity _ball_max_height)) (Math|Float|Sqrt (|((2*(disZ-h))/g) _gravity _ball_max_height (LocalVariables|GetZdisplacement)))))))
  (return (+ _output_get _output_get_2)))

(fn Player02Launch
  (bind _player_02_aimtarget (Variables|Default|GetPlayer_02_AimTarget))
  (bind _tennisball (Variables|Default|GetTennisBall))
  (bind _ball_max_height (Variables|Exposed|GetBall%20Max%20Height))
  (bind _gravity (Variables|Math|GetGravity))
  (bind _returnvalue (Transformation|GetWorldLocation _player_02_aimtarget))
  (bind _returnvalue_2 (Transformation|GetWorldLocation _tennisball))
  (LocalVariables|SetZdisplacement (- (.z _returnvalue) (.z _returnvalue_2)))
  (LocalVariables|SetXYdisplacement (Math|Vector|MakeVector (- (.x _returnvalue) (.x _returnvalue_2)) (- (.y _returnvalue) (.y _returnvalue_2)) 0.0))
  (bind _output_get (LocalVariables|SetZVelocity (* (Math|Vector|VectorUp) (Math|Float|Sqrt (|(((0-2)*g)*h) _gravity _ball_max_height)))))
  (bind _output_get_2 (LocalVariables|SetXYVelocity (/ (LocalVariables|GetXYdisplacement) (+ (Math|Float|Sqrt (|(((0-2)*h)/g) _gravity _ball_max_height)) (Math|Float|Sqrt (|((2*(disZ-h))/g) _gravity _ball_max_height (LocalVariables|GetZdisplacement)))))))
  (return (+ _output_get _output_get_2)))