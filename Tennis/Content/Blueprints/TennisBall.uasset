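; Tennis ball Blueprint that moves the ball between two players, with a bounce at the hitter's aim target.
; Each player's hit event chains two rate-scaled timelines, lerping the ball from hitter to aim target, then to the opponent's position target.
; A separate Launch event enables physics and sets a velocity calculated from max height, gravity and Player 1's aim target.
; Physics starts disabled, and older AddForce attempts remain unconnected.
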(event Custom|Player_02_Hit
  (bind _tennisball (Variables|Default|GetTennisBall))
  (bind _player_02_aimtarget (Variables|Default|GetPlayer_02_AimTarget))
  (bind _returnvalue (Transformation|GetWorldLocation _player_02_aimtarget))
  ;[1 1 1] Less Terrible
  (Components|Timeline|SetPlayRate (Variables|Default|GetPlayer02%20Hit) (Variables|Default|GetHit%20Speed))
  (Components|Timeline|SetPlayRate (Variables|Default|GetPlayer02%20Bounce) (Variables|Default|GetBounce%20Speed))
  (bind _before_bounce (Timeline|Player02%20Hit Play)
    (:Update
      (Transformation|SetWorldLocation _tennisball (Math|Vector|Lerp(Vector) (Transformation|GetWorldLocation (Variables|Default|GetPlayer_02)) _returnvalue _before_bounce) false false))
    (:Finished
      (bind _after_bounce (Timeline|Player02%20Bounce Play)
        (:Update
          (Transformation|SetWorldLocation _tennisball (Math|Vector|Lerp(Vector) _returnvalue (Transformation|GetWorldLocation (Variables|Default|GetPlayer_01_PositionTarget)) _after_bounce) false false))))))

(event Custom|Launch
  (bind _player_01_aimtarget (Variables|Default|GetPlayer_01_AimTarget))
  (bind _player_01 (Variables|Default|GetPlayer_01))
  (bind _ball_target_point (Variables|Physics|GetBall%20Target%20Point))
  (bind _ball_max_height (Variables|Ball|GetBall%20Max%20Height))
  (bind _player_01_aimtarget_2 (Variables|Default|GetPlayer_01_AimTarget))
  (bind _player_01_2 (Variables|Default|GetPlayer_01))
  (bind _tennisball (Variables|Default|GetTennisBall))
  (bind _ball_max_height_2 (Variables|Ball|GetBall%20Max%20Height))
  (bind _gravity (Variables|BallUp|GetGravity))
  (bind _returnvalue (Transformation|GetWorldLocation _player_01_aimtarget_2))
  (bind _returnvalue_2 (Transformation|GetWorldLocation _player_01_aimtarget))
  (bind _returnvalue_3 (Transformation|GetWorldLocation _player_01))
  (bind _returnvalue_4 (Transformation|GetWorldLocation _player_01_2))
  (bind _returnvalue_5 (|2*(P-h)/g _ball_max_height _gravity _ball_target_point))
  (bind _returnvalue_6 (|(2*h)/g _ball_max_height_2 _gravity))
  (bind _returnvalue_7 (Math|Float|Sqrt _returnvalue_5))
  (bind _returnvalue_8 (* _returnvalue_6 -1.0))
  (bind _returnvalue_9 (Math|Float|Sqrt _returnvalue_8))
  (bind _returnvalue_10 (+ _returnvalue_9 _returnvalue_7))
  ;[1 1 1] Calculating Velocity
  (Variables|Default|SetBall%20Velocity%20Z (Math|Float|Sqrt (|x*g*h (Variables|Ball|GetBall%20Max%20Height) (Variables|BallUp|GetGravity) -2.0)))
  (Variables|Default|SetBall%20Velocity%20XY (/ (Math|Vector|Distance(Vector) (Math|Vector|MakeVector (.x _returnvalue_4) (.y _returnvalue_4) 0.0) (Math|Vector|MakeVector (.x _returnvalue) (.y _returnvalue) 0.0)) _returnvalue_10))
  (Variables|Default|SetDisplacement%20XYZ "0, 0, 0")
  (Physics|SetSimulatePhysics _tennisball true)
  (Class|PrimitiveComponent|SetAllPhysicsLinearVelocity _tennisball (+ (/ (Math|Vector|MakeVector (- (.x _returnvalue_2) (.x _returnvalue_3)) (- (.y _returnvalue_2) (.y _returnvalue_3)) 0.0) _returnvalue_10) (* (Math|Vector|MakeVector 0.0 0.0 _returnvalue_9) (* (Math|Trig|Sin(Degrees) (Variables|BallUp|GetGravity)) -1.0))) false))

(event Custom|Player_01%20Hit
  (bind _tennisball (Variables|Default|GetTennisBall))
  (bind _player_01_aimtarget (Variables|Default|GetPlayer_01_AimTarget))
  (bind _returnvalue (Transformation|GetWorldLocation _player_01_aimtarget))
  ;[1 1 1] Less Terrible
  (Components|Timeline|SetPlayRate (Variables|Default|GetPlayer01%20Hit) (Variables|Default|GetHit%20Speed))
  (Components|Timeline|SetPlayRate (Variables|Default|GetPlayer01%20Bounce) (Variables|Default|GetBounce%20Speed))
  (bind _before_bounce (Timeline|Player01%20Hit Play)
    (:Update
      (Transformation|SetWorldLocation _tennisball (Math|Vector|Lerp(Vector) (Transformation|GetWorldLocation (Variables|Default|GetPlayer_01)) _returnvalue _before_bounce) false false))
    (:Finished
      (bind _after_bounce (Timeline|Player01%20Bounce Play)
        (:Update
          (Transformation|SetWorldLocation _tennisball (Math|Vector|Lerp(Vector) _returnvalue (Transformation|GetWorldLocation (Variables|Default|GetPlayer_02_PositionTarget)) _after_bounce) false false))))))

(event EventBeginPlay
  (Physics|SetSimulatePhysics (Variables|Default|GetTennisBall) false))

(fn ConstructionScript)