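; Tennis ball actor that handles player hits, bounces and serves by toggling physics and setting computed velocities.
; Hit events use BallLaunch's kinematic arc math, from gravity and a max height, to reach each player's aim target, then swap trail particles.
; Bounce and serve compute velocity and wait time, then either freeze the ball or, for a non-catch serve, trigger Player 01's hit.
; Aim-target timeline logic is unconnected.
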(event Custom|BounceBall
  (bind _ball (Variables|Default|GetBall))
  (bind _tennisball (Variables|/Game/LiveProxy/Tennis/Blueprints/Ball.Ball_C|GetTennisBall _ball))
  (bind (_return _waittime) (CallFunction|BallBounce))
  (Physics|SetSimulatePhysics _tennisball true)
  (Class|PrimitiveComponent|SetAllPhysicsLinearVelocity _tennisball _return false)
  (Utilities|FlowControl|Delay _waittime)
  (Physics|SetSimulatePhysics _tennisball false))

(event Custom|Player02_Hit
  (bind _ball (Variables|Default|GetBall))
  (bind _tennisball (Variables|/Game/LiveProxy/Tennis/Blueprints/Ball.Ball_C|GetTennisBall _ball))
  (bind _return (CallFunction|BallLaunch (Variables|Default|GetPlayer_02_AimTarget)))
  (Physics|SetSimulatePhysics _tennisball true)
  (Class|PrimitiveComponent|SetAllPhysicsLinearVelocity _tennisball _return false)
  (CallFunction|SwapParticleVisibility (Variables|/Game/LiveProxy/Tennis/Blueprints/Ball.Ball_C|GetTennisBall_Player02_Trail _ball) (Variables|/Game/LiveProxy/Tennis/Blueprints/Ball.Ball_C|GetTennisBall_Player01_Trail _ball)))

(event Custom|Player01_Hit
  (bind _ball (Variables|Default|GetBall))
  (bind _tennisball (Variables|/Game/LiveProxy/Tennis/Blueprints/Ball.Ball_C|GetTennisBall _ball))
  (bind _return (CallFunction|BallLaunch (Variables|Default|GetPlayer_01_AimTarget)))
  (Physics|SetSimulatePhysics _tennisball true)
  (Class|PrimitiveComponent|SetAllPhysicsLinearVelocity _tennisball _return false)
  (CallFunction|SwapParticleVisibility (Variables|/Game/LiveProxy/Tennis/Blueprints/Ball.Ball_C|GetTennisBall_Player01_Trail _ball) (Variables|/Game/LiveProxy/Tennis/Blueprints/Ball.Ball_C|GetTennisBall_Player02_Trail _ball)))

(event Custom|ServeBall
  (params (isCatchThrow :type Boolean))
  (bind _ball (Variables|Default|GetBall))
  (bind _tennisball (Variables|/Game/LiveProxy/Tennis/Blueprints/Ball.Ball_C|GetTennisBall _ball))
  (bind (_return _waittime) (CallFunction|BallServeThrow 2.5e+02))
  (Physics|SetSimulatePhysics _tennisball true)
  (Class|PrimitiveComponent|SetAllPhysicsLinearVelocity _tennisball _return false)
  (if isCatchThrow
    (Utilities|FlowControl|Delay _waittime)
    (Physics|SetSimulatePhysics _tennisball false)
    (else
      (Utilities|FlowControl|Delay (/ _waittime 1.7))
      (CallFunction|Player01Hit))))

(event EventBeginPlay
  (Physics|SetSimulatePhysics (Variables|/Game/LiveProxy/Tennis/Blueprints/Ball.Ball_C|GetTennisBall (Variables|Default|GetBall)) false))

(fn ConstructionScript)

(fn BallLaunch
  (params (TargetObject :type Scene%20Component%20Object%20Reference))
  (bind _returnvalue (Transformation|GetWorldLocation TargetObject))
  (bind _ball (Variables|Default|GetBall))
  (bind _ball_max_height (Variables|Exposed|GetBall%20Max%20Height))
  (bind _gravity (Variables|Math|GetGravity))
  (bind _tennisball (Variables|/Game/LiveProxy/Tennis/Blueprints/Ball.Ball_C|GetTennisBall _ball))
  (bind _returnvalue_2 (Transformation|GetWorldLocation _tennisball))
  (LocalVariables|SetZdisplacement (- (.z _returnvalue) (.z _returnvalue_2)))
  (LocalVariables|SetXYdisplacement (Math|Vector|MakeVector (- (.x _returnvalue) (.x _returnvalue_2)) (- (.y _returnvalue) (.y _returnvalue_2)) 0.0))
  (return (+ (* (Math|Vector|VectorUp) (Math|Float|Sqrt (|(((0-2)*g)*h) _gravity _ball_max_height))) (/ (LocalVariables|GetXYdisplacement) (+ (Math|Float|Sqrt (|(((0-2)*h)/g) _gravity _ball_max_height)) (Math|Float|Sqrt (|((2*(disZ-h))/g) _gravity _ball_max_height (LocalVariables|GetZdisplacement))))))))

(fn Player02Launch
  (bind _player_02_aimtarget (Variables|Default|GetPlayer_02_AimTarget))
  (bind _ball (Variables|Default|GetBall))
  (bind _ball_max_height (Variables|Exposed|GetBall%20Max%20Height))
  (bind _gravity (Variables|Math|GetGravity))
  (bind _returnvalue (Transformation|GetWorldLocation _player_02_aimtarget))
  (bind _tennisball (Variables|/Game/LiveProxy/Tennis/Blueprints/Ball.Ball_C|GetTennisBall _ball))
  (bind _returnvalue_2 (Transformation|GetWorldLocation _tennisball))
  (LocalVariables|SetZdisplacement (- (.z _returnvalue) (.z _returnvalue_2)))
  (LocalVariables|SetXYdisplacement (Math|Vector|MakeVector (- (.x _returnvalue) (.x _returnvalue_2)) (- (.y _returnvalue) (.y _returnvalue_2)) 0.0))
  (bind _output_get (LocalVariables|SetZVelocity (* (Math|Vector|VectorUp) (Math|Float|Sqrt (|(((0-2)*g)*h) _gravity _ball_max_height)))))
  (bind _output_get_2 (LocalVariables|SetXYVelocity (/ (LocalVariables|GetXYdisplacement) (+ (Math|Float|Sqrt (|(((0-2)*h)/g) _gravity _ball_max_height)) (Math|Float|Sqrt (|((2*(disZ-h))/g) _gravity _ball_max_height (LocalVariables|GetZdisplacement)))))))
  (return (+ _output_get _output_get_2)))

(fn SwapParticleVisibility
  (params (ParticleOn :type Particle%20System%20Component%20Object%20Reference) (ParticleOff :type Particle%20System%20Component%20Object%20Reference))
  (Components|Activation|SetActive ParticleOn false true)
  (Rendering|SetVisibility ParticleOn false false)
  (Components|Activation|SetActive ParticleOff true false)
  (Rendering|SetVisibility ParticleOff true false))

(fn BallBounce
  (bind _ball (Variables|Default|GetBall))
  (bind _tennisball (Variables|/Game/LiveProxy/Tennis/Blueprints/Ball.Ball_C|GetTennisBall _ball))
  (bind _returnvalue (Transformation|GetWorldLocation _tennisball))
  (bind _output_get (LocalVariables|SetInitVelocity (Math|Vector|MakeVector 0.0 0.0 (* -1 (Math|Float|Sqrt (- 0.0 (* 2.0 (/ (Variables|Math|GetGravity) 2.0) (.z _returnvalue))))))))
  (return _output_get (- (Math|Float|Sqrt (Math|Float|Absolute(Float) (|((2*d)/g) (.z _returnvalue) (/ (Variables|Math|GetGravity) 2.0)))) 0.04)))

(fn BallServeThrow
  (params (ThrowHeight :type Float%20%28single-precision%29))
  (bind _gravity (Variables|Math|GetGravity))
  (bind _returnvalue (/ _gravity 2.0))
  (return (Math|Vector|MakeVector 0.0 0.0 (Math|Float|Sqrt (- 0.0 (* 2.0 (Variables|Math|GetGravity) ThrowHeight)))) (- (Math|Float|Sqrt (+ (|(0-((2*d)/g)) ThrowHeight _returnvalue) (Math|Float|Absolute(Float) (|((2*d)/g) ThrowHeight _returnvalue)))) 0.04)))